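; Ball actor that travels in a random direction and bounces off whatever it hits.
; BeginPlay picks a random unit vector, then normalizes it in 2D as the travel direction.
; Each Tick sweeps the actor by direction times speed, without delta time scaling, and reflects the direction about the hit normal on a blocking hit.
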(event EventTick
  (params (DeltaSeconds :type Float%20%28single-precision%29))
  (bind _sweephitresult (Transformation|AddActorWorldOffset (* (Variables|Default|GetDirection) (Variables|Default|GetSpeed)) true))
  (if (.bBlockingHit (Collision|BreakHitResult _sweephitresult))
    (Variables|Default|SetDirection (Math|Vector|GetReflectionVector (Variables|Default|GetDirection) (.Normal (Collision|BreakHitResult _sweephitresult))))))

(event EventBeginPlay
  (Variables|Default|SetDirection (Class|KismetMathLibrary|VectorNormal2D (Math|Random|RandomUnitVector) 0.0001)))

(fn ConstructionScript)